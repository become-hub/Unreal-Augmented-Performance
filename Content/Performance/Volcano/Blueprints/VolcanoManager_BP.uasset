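; Volcano manager actor that shifts the volcano's lava, smoke and audio between five escalating states.
; Each state switches on cumulative Niagara smoke stages and sets targets for a timeline that lerps lava radius and emissive on a dynamic material, plus an audio blend parameter.
; State changes arriving while the timeline plays are ignored.
; Either VR grab input clears a timer and opens the WaitingRoom level.
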(event Custom|VolcanUpdate
  (params (CurrentState :type E_States%20Enum :default "NewEnumerator0"))
  (bind _volcanomi (Variables|Default|GetVolcanoMI))
  (if (not (Variables|Default|GetIsPlaying))
    (Variables|Default|SetIsPlaying true)
    (Variables|Default|SetCurrentState CurrentState)
    (CallFunction|SetNiagaraBool)
    (switch Utilities|FlowControl|Switch|SwitchonE_States (Variables|Default|GetCurrentState)
      (:NewEnumerator0
        (Variables|Default|SetTargetLavaRadius 0.0)
        (Variables|Default|SetCurrentVolume 0.8)
        (bind _alpha (Timeline|LavaTimeline PlayFromStart)
          (:Update
            (Variables|Default|SetAlpha _alpha)
            (Rendering|Material|SetScalarParameterValue _volcanomi "LavaRadius" (Math|Float|Lerp (Variables|Default|GetCurrentLavaRadius) (Variables|Default|GetTargetLavaRadius) (Variables|Default|GetAlpha)) :!class /Script/Engine.MaterialInstanceDynamic)
            (Rendering|Material|SetScalarParameterValue _volcanomi "EmissiveIntensity" (Math|Float|Lerp (Variables|Default|GetCurrentLavaRadius) (Variables|Default|GetTargetLavaRadius) (Variables|Default|GetAlpha)) :!class /Script/Engine.MaterialInstanceDynamic)
            (Audio|Parameter|SetFloatParameter (Variables|Default|GetBlendVolcano) "BlendWether" (Math|Float|Lerp (Variables|Default|GetLastVolume) (Variables|Default|GetCurrentVolume) (Variables|Default|GetAlpha)) :!class /Script/Engine.AudioComponent))
          (:Finished
            (Variables|Default|SetIsPlaying false)
            (Variables|Default|SetCurrentLavaRadius (Variables|Default|GetTargetLavaRadius))
            (Variables|Default|SetLastVolume (Variables|Default|GetCurrentVolume)))))
      (:NewEnumerator1
        (Variables|Default|SetTargetLavaRadius 0.0)
        (Variables|Default|SetCurrentVolume 1.0)
        (Timeline|LavaTimeline PlayFromStart))
      (:NewEnumerator2
        (Variables|Default|SetTargetLavaRadius 0.0)
        (Variables|Default|SetCurrentVolume 2.0)
        (Timeline|LavaTimeline PlayFromStart))
      (:NewEnumerator3
        (Variables|Default|SetTargetLavaRadius 1.0)
        (Variables|Default|SetCurrentVolume 3.0)
        (Timeline|LavaTimeline PlayFromStart))
      (:NewEnumerator4
        (Variables|Default|SetTargetLavaRadius 1.0)
        (Variables|Default|SetCurrentVolume 3.9)
        (Timeline|LavaTimeline PlayFromStart)))))

(event Custom|CustomEvent
  (params (NewState :type E_States%20Enum :default "NewEnumerator0"))
  (CallFunction|VolcanUpdate NewState)
  (Development|PrintString (Utilities|String|Append "CHANGE STATE EVENT IN WM: " (Utilities|String|EnumtoString NewState))))

(event Input|EnhancedActionEvents|EnhancedInputActionIA_Grab_Left_Pressed
  (params (ActionValue :type Float%20%28double-precision%29) (ElapsedSeconds :type Float%20%28double-precision%29) (TriggeredSeconds :type Float%20%28double-precision%29) (InputAction :type Input%20Action%20Object%20Reference :default "/Game/VRTemplate/Input/Actions/IA_Grab_Left_Pressed.IA_Grab_Left_Pressed"))
  (Utilities|Time|ClearandInvalidateTimerbyHandle (Variables|Default|GetTimerHandler))
  (Game|OpenLevel(byName) "WaitingRoom"))

(event Input|EnhancedActionEvents|EnhancedInputActionIA_Grab_Right_Pressed
  (params (ActionValue :type Float%20%28double-precision%29) (ElapsedSeconds :type Float%20%28double-precision%29) (TriggeredSeconds :type Float%20%28double-precision%29) (InputAction :type Input%20Action%20Object%20Reference :default "/Game/VRTemplate/Input/Actions/IA_Grab_Right_Pressed.IA_Grab_Right_Pressed"))
  (Utilities|Time|ClearandInvalidateTimerbyHandle (Variables|Default|GetTimerHandler))
  (Game|OpenLevel(byName) "WaitingRoom"))

(event EventBeginPlay
  (bind _returnvalue (Rendering|Material|CreateDynamicMaterialInstance (Variables|Default|GetSM_Volcano) 0 "/Game/Performance/Volcano/Environment/LandscapeCollection/Materials/MASTER/M_Volcano.M_Volcano" "None" :!class /Script/Engine.PrimitiveComponent))
  (Variables|Default|SetVolcanoMI _returnvalue)
  (Audio|Components|Audio|Play (Variables|Default|GetBlendVolcano) 0.0))

(fn ConstructionScript
  (bind _returnvalue (Rendering|Material|CreateDynamicMaterialInstance (Variables|Default|GetSM_Volcano) 0 "/Game/Performance/Volcano/Environment/LandscapeCollection/Materials/MASTER/M_Volcano.M_Volcano" "None" :!class /Script/Engine.PrimitiveComponent))
  (Variables|Default|SetVolcanoMI _returnvalue))

(fn SetNiagaraBool
  (bind _ns_volcanosmoke (Variables|Default|GetNS_VolcanoSmoke))
  (bind _ns_volcanosmoke_2 (Variables|Default|GetNS_VolcanoSmoke))
  (Class|NiagaraComponent|SetVariableBool _ns_volcanosmoke_2 "user.Stage1" false)
  (Class|NiagaraComponent|SetVariableBool _ns_volcanosmoke_2 "user.Stage2" false)
  (Class|NiagaraComponent|SetVariableBool _ns_volcanosmoke_2 "user.Stage3" false)
  (Class|NiagaraComponent|SetVariableBool _ns_volcanosmoke_2 "user.Stage4" false)
  (switch Utilities|FlowControl|Switch|SwitchonE_States (Variables|Default|GetCurrentState)
    (:NewEnumerator0
      (return))
    (:NewEnumerator1
      (Class|NiagaraComponent|SetVariableBool _ns_volcanosmoke "user.Stage1" true)
      (return))
    (:NewEnumerator2
      (Class|NiagaraComponent|SetVariableBool _ns_volcanosmoke "user.Stage2" true)
      (Class|NiagaraComponent|SetVariableBool _ns_volcanosmoke "user.Stage1" true)
      (return))
    (:NewEnumerator3
      (Class|NiagaraComponent|SetVariableBool _ns_volcanosmoke "user.Stage3" true)
      (Class|NiagaraComponent|SetVariableBool _ns_volcanosmoke "user.Stage2" true)
      (Class|NiagaraComponent|SetVariableBool _ns_volcanosmoke "user.Stage1" true)
      (return))
    (:NewEnumerator4
      (Class|NiagaraComponent|SetVariableBool _ns_volcanosmoke "user.Stage4" true)
      (Class|NiagaraComponent|SetVariableBool _ns_volcanosmoke "user.Stage3" true)
      (Class|NiagaraComponent|SetVariableBool _ns_volcanosmoke "user.Stage2" true)
      (Class|NiagaraComponent|SetVariableBool _ns_volcanosmoke "user.Stage1" true)
      (return))))