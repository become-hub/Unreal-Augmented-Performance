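; Weather manager for the ocean map that transitions between five sea states on state-change events.
; It snapshots current values, then a shared timeline lerps preset colors, foam, height, fog, rain, sun intensity and cloud opacity through MPC_Weather, NPC_OceanWeather and scene actors.
; The same timeline blends the BlendOcean audio parameter using volumes from SeaParams_DT, loaded at BeginPlay.
; Either grab input opens the WaitingRoom level.
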(event Custom|WeatherUpdate
  (params (WeatherCondition :type E_States%20Enum :default "NewEnumerator0"))
  (if (not (Variables|Default|GetisPlaying))
    (Variables|Default|SetCurrentState WeatherCondition)
    (CallFunction|GetCurrentWeatherState)
    (CallFunction|GetCurrentLightingSettings)
    (switch Utilities|FlowControl|Switch|SwitchonE_States (Variables|Default|GetCurrentState)
      (:NewEnumerator0
        (Variables|Params|SetCurrentBW (.volume (Variables|Params|GetParamsP-2)))
        (bind _alpha (Timeline|Timeline_0 PlayFromStart)
          (:Update
            (Variables|Default|SetAlpha _alpha)
            (switch Utilities|FlowControl|Switch|SwitchonE_States (Variables|Default|GetCurrentState)
              (:NewEnumerator0
                (CallFunction|UpdateWeather (Variables|Default|GetAlpha) "(R=0.095307,G=0.467784,B=1.000000,A=1.000000)" "(R=1.000000,G=1.000000,B=0.930111,A=1.000000)" "(R=0.341914,G=0.651406,B=0.846873,A=1.000000)" "(R=0.039546,G=0.198069,B=0.417885,A=1.000000)" 0.0 0.01 0.0 0 0.0)
                (CallFunction|UpdateSky 6.0 0.7 (Variables|Default|GetAlpha)))
              (:NewEnumerator1
                (CallFunction|UpdateWeather (Variables|Default|GetAlpha) "(R=0.095307,G=0.467784,B=1.000000,A=1.000000)" "(R=1.000000,G=1.000000,B=0.930111,A=1.000000)" "(R=0.341914,G=0.651406,B=0.846873,A=1.000000)" "(R=0.039546,G=0.198069,B=0.417885,A=1.000000)" 1.5 0.01 0.0 0 1e+02)
                (CallFunction|UpdateSky 6.0 0.7 (Variables|Default|GetAlpha)))
              (:NewEnumerator2
                (CallFunction|UpdateWeather (Variables|Default|GetAlpha) "(R=0.058822,G=0.288710,B=0.617188,A=1.000000)" "(R=1.000000,G=1.000000,B=0.930111,A=1.000000)" "(R=0.341914,G=0.651406,B=0.846873,A=1.000000)" "(R=0.039546,G=0.198069,B=0.417885,A=1.000000)" 2.0 0.01 0.0 25 2e+02)
                (CallFunction|UpdateSky 6.0 0.7 (Variables|Default|GetAlpha)))
              (:NewEnumerator3
                (CallFunction|UpdateWeather (Variables|Default|GetAlpha) "(R=0.058822,G=0.288710,B=0.617188,A=1.000000)" "(R=0.578125,G=0.578125,B=0.537720,A=1.000000)" "(R=0.341914,G=0.651406,B=0.846873,A=1.000000)" "(R=0.039546,G=0.198069,B=0.417885,A=1.000000)" 4.0 0.01 0.0 50 3e+02)
                (CallFunction|UpdateSky 1.0 2.0 (Variables|Default|GetAlpha)))
              (:NewEnumerator4
                (CallFunction|UpdateWeather (Variables|Default|GetAlpha) "(R=0.011913,G=0.058473,B=0.125000,A=1.000000)" "(R=0.578125,G=0.578125,B=0.537720,A=1.000000)" "(R=0.341914,G=0.651406,B=0.846873,A=1.000000)" "(R=0.039546,G=0.198069,B=0.417885,A=1.000000)" 4.0 0.25 1e+03 100 4e+02)
                (CallFunction|UpdateSky 0.1 4.0 (Variables|Default|GetAlpha))))
            (Audio|Parameter|SetFloatParameter (Variables|Default|GetBlendOcean) "BlendWeather" (Math|Float|Lerp (Variables|Params|GetLastBW) (Variables|Params|GetCurrentBW) (Variables|Default|GetAlpha)) :!class /Script/Engine.AudioComponent)
            (Variables|Default|SetisPlaying false))
          (:Finished
            (Variables|Params|SetLastBW (Variables|Params|GetCurrentBW)))))
      (:NewEnumerator1
        (Variables|Params|SetCurrentBW (.volume (Variables|Params|GetParamsP-1)))
        (Timeline|Timeline_0 PlayFromStart))
      (:NewEnumerator2
        (Variables|Params|SetCurrentBW (.volume (Variables|Params|GetParamsP0)))
        (Timeline|Timeline_0 PlayFromStart))
      (:NewEnumerator3
        (Variables|Params|SetCurrentBW (.volume (Variables|Params|GetParamsP1)))
        (Timeline|Timeline_0 PlayFromStart))
      (:NewEnumerator4
        (Variables|Params|SetCurrentBW (.volume (Variables|Params|GetParamsP2)))
        (Timeline|Timeline_0 PlayFromStart)))))

(event Input|EnhancedActionEvents|EnhancedInputActionIA_Grab_Left_Pressed
  (params (ActionValue :type Float%20%28double-precision%29) (ElapsedSeconds :type Float%20%28double-precision%29) (TriggeredSeconds :type Float%20%28double-precision%29) (InputAction :type Input%20Action%20Object%20Reference :default "/Game/VRTemplate/Input/Actions/IA_Grab_Left_Pressed.IA_Grab_Left_Pressed"))
  (Utilities|Time|ClearandInvalidateTimerbyHandle (Variables|Default|GetTimerHandler))
  (Game|OpenLevel(byName) "WaitingRoom"))

(event Input|EnhancedActionEvents|EnhancedInputActionIA_Grab_Right_Pressed
  (params (ActionValue :type Float%20%28double-precision%29) (ElapsedSeconds :type Float%20%28double-precision%29) (TriggeredSeconds :type Float%20%28double-precision%29) (InputAction :type Input%20Action%20Object%20Reference :default "/Game/VRTemplate/Input/Actions/IA_Grab_Right_Pressed.IA_Grab_Right_Pressed"))
  (Utilities|Time|ClearandInvalidateTimerbyHandle (Variables|Default|GetTimerHandler))
  (Game|OpenLevel(byName) "WaitingRoom"))

(event EventChangeStateEvent
  (params (NewState :type E_States%20Enum :default "NewEnumerator0"))
  (Development|PrintString (Utilities|String|Append "CHANGE STATE EVENT IN WM: " (Utilities|String|EnumtoString NewState)))
  (CallFunction|WeatherUpdate NewState))

(event EventBeginPlay
  (|InitializeParams))

(fn ConstructionScript)

(fn UpdateWeather
  (params (Alpha :type Float%20%28double-precision%29) (EnviromentColor :type Linear%20Color%20Structure) (FogColor :type Linear%20Color%20Structure) (WaterDeepColor :type Linear%20Color%20Structure) (WaterShallowColor :type Linear%20Color%20Structure) (FoamIntensity :type Float%20%28double-precision%29) (FogOpacity :type Float%20%28double-precision%29) (RainSpawnCount :type Float%20%28double-precision%29) (FoamSpawnCount :type Integer) (Height :type Float%20%28double-precision%29))
  (Development|PrintString (Utilities|String|ToString(Float) Alpha) false false)
  (Utilities|FlowControl|Sequence
    (:then_0
      (Rendering|Material|SetVectorParameterValue "/Game/Performance/OceanMap/Materials/MPC_Weather.MPC_Weather" "EnviromentColor" (Math|Color|Lerp(LinearColor) (Variables|Default|GetTempEnviromentColor) EnviromentColor Alpha) :!class /Script/Engine.KismetMaterialLibrary)
      (Rendering|Material|SetVectorParameterValue "/Game/Performance/OceanMap/Materials/MPC_Weather.MPC_Weather" "FogColor" (Math|Color|Lerp(LinearColor) (Variables|Default|GetTempFogColor) FogColor Alpha) :!class /Script/Engine.KismetMaterialLibrary)
      (Rendering|Material|SetVectorParameterValue "/Game/Performance/OceanMap/Materials/MPC_Weather.MPC_Weather" "WaterDeepColor" (Math|Color|Lerp(LinearColor) (Variables|Default|GetTempWaterDeepColor) WaterDeepColor Alpha) :!class /Script/Engine.KismetMaterialLibrary)
      (Rendering|Material|SetVectorParameterValue "/Game/Performance/OceanMap/Materials/MPC_Weather.MPC_Weather" "WaterShallowColor" (Math|Color|Lerp(LinearColor) (Variables|Default|GetTempWaterShallowColor) WaterShallowColor Alpha) :!class /Script/Engine.KismetMaterialLibrary))
    (:then_1
      (Rendering|Material|SetScalarParameterValue "/Game/Performance/OceanMap/Materials/MPC_Weather.MPC_Weather" "FoamIntensity" (Math|Float|Lerp (Variables|Default|GetTempFoamIntensity) FoamIntensity Alpha) :!class /Script/Engine.KismetMaterialLibrary)
      (Rendering|Material|SetScalarParameterValue "/Game/Performance/OceanMap/Materials/MPC_Weather.MPC_Weather" "Height" (Math|Float|Lerp (Variables|Default|GetTempHeight) Height Alpha) :!class /Script/Engine.KismetMaterialLibrary)
      (Class|ExponentialHeightFogComponent|SetFogDensity (Variables|/Script/Engine.ExponentialHeightFog|GetComponent (Variables|Default|GetFog)) (Math|Float|Lerp (Variables|Default|GetTempFogDensity) FogOpacity Alpha)))
    (:then_2
      (bind _returnvalue (Class|NiagaraFunctionLibrary|GetNiagaraParameterCollection "/Game/Performance/OceanMap/VFX/NPC_OceanWeather.NPC_OceanWeather"))
      (Effects|Components|ParticleSystem|SetFloatParameter _returnvalue "RainSpawnCount" (Math|Float|Lerp (Variables|Default|GetTempRainSpawnCount) RainSpawnCount Alpha))
      (bind _returnvalue_2 (Class|NiagaraFunctionLibrary|GetNiagaraParameterCollection "/Game/Performance/OceanMap/VFX/NPC_OceanWeather.NPC_OceanWeather"))
      (Effects|Components|ParticleSystem|SetIntParameter _returnvalue_2 "FoamSpawnCount" FoamSpawnCount))))

(fn GetCurrentWeatherState
  (Utilities|FlowControl|Sequence
    (:then_0
      (bind _returnvalue (Rendering|Material|GetVectorParameterValue "/Game/Performance/OceanMap/Materials/MPC_Weather.MPC_Weather" "EnviromentColor" :!class /Script/Engine.KismetMaterialLibrary))
      (Variables|Default|SetTempEnviromentColor _returnvalue)
      (bind _returnvalue_2 (Rendering|Material|GetVectorParameterValue "/Game/Performance/OceanMap/Materials/MPC_Weather.MPC_Weather" "FogColor" :!class /Script/Engine.KismetMaterialLibrary))
      (Variables|Default|SetTempFogColor _returnvalue_2)
      (bind _returnvalue_3 (Rendering|Material|GetVectorParameterValue "/Game/Performance/OceanMap/Materials/MPC_Weather.MPC_Weather" "WaterDeepColor" :!class /Script/Engine.KismetMaterialLibrary))
      (Variables|Default|SetTempWaterDeepColor _returnvalue_3)
      (bind _returnvalue_4 (Rendering|Material|GetVectorParameterValue "/Game/Performance/OceanMap/Materials/MPC_Weather.MPC_Weather" "WaterShallowColor" :!class /Script/Engine.KismetMaterialLibrary))
      (Variables|Default|SetTempWaterShallowColor _returnvalue_4))
    (:then_1
      (bind _returnvalue_5 (Rendering|Material|GetScalarParameterValue "/Game/Performance/OceanMap/Materials/MPC_Weather.MPC_Weather" "FoamIntensity" :!class /Script/Engine.KismetMaterialLibrary))
      (Variables|Default|SetTempFoamIntensity _returnvalue_5)
      (bind _returnvalue_6 (Rendering|Material|GetScalarParameterValue "/Game/Performance/OceanMap/Materials/MPC_Weather.MPC_Weather" "Height" :!class /Script/Engine.KismetMaterialLibrary))
      (Variables|Default|SetTempHeight _returnvalue_6)
      (Variables|Default|SetTempFogDensity (Variables|/Script/Engine.ExponentialHeightFogComponent|GetFogDensity (Variables|/Script/Engine.ExponentialHeightFog|GetComponent (Variables|Default|GetFog)))))
    (:then_2
      (bind _returnvalue_7 (Class|NiagaraFunctionLibrary|GetNiagaraParameterCollection "/Game/Performance/OceanMap/VFX/NPC_OceanWeather.NPC_OceanWeather"))
      (bind _returnvalue_8 (Class|NiagaraParameterCollectionInstance|GetFloatParameter _returnvalue_7 "RainSpawnCount"))
      (Variables|Default|SetTempRainSpawnCount _returnvalue_8)
      (Class|NiagaraFunctionLibrary|GetNiagaraParameterCollection "/Game/Performance/OceanMap/VFX/NPC_OceanWeather.NPC_OceanWeather"))))

(fn GetCurrentLightingSettings
  (Variables|Default|SetTempLightintensity (Variables|/Script/Engine.LightComponentBase|GetIntensity (Variables|/Script/Engine.Light|GetLightComponent (Variables|Default|GetDirectionallight))))
  (Variables|Default|SetTempCloudOpacity (Variables|/Engine/EngineSky/BP_Sky_Sphere.BP_Sky_Sphere_C|GetCloud%20opacity (Variables|Default|GetBP_Skysphere))))

(fn UpdateSky
  (params (Lightintensity :type Float%20%28double-precision%29) (CloudOpacity :type Float%20%28double-precision%29) (Alpha :type Float%20%28double-precision%29))
  (bind _bp_skysphere (Variables|Default|GetBP_Skysphere))
  (Rendering|Components|Light|SetIntensity (Variables|/Script/Engine.Light|GetLightComponent (Variables|Default|GetDirectionallight)) (Math|Float|Lerp (Variables|Default|GetTempLightintensity) Lightintensity (Variables|Default|GetAlpha)))
  (bind _output_get (Variables|/Engine/EngineSky/BP_Sky_Sphere.BP_Sky_Sphere_C|SetCloud%20opacity _bp_skysphere (Math|Float|Lerp (Variables|Default|GetTempCloudOpacity) CloudOpacity (Variables|Default|GetAlpha))))
  (Rendering|Material|SetScalarParameterValue (Variables|/Engine/EngineSky/BP_Sky_Sphere.BP_Sky_Sphere_C|GetSky%20material _bp_skysphere) "Cloud opacity" _output_get :!class /Script/Engine.MaterialInstanceDynamic))