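; Construction-script tool that scatters or bends static meshes along a spline, spaced uniformly by count or sequentially by mesh width.
; GetMesh randomly picks from Start, Fill and End sets, reusing one instanced component per mesh unless curving uses spline mesh components.
; GetTransform samples the spline, then applies optional local transforms, seeded random variation and downward-trace terrain snapping.
; Optional settings turn each piece toward the next or limit rotation to yaw.
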(event EventBeginPlay)

(event EventActorBeginOverlap
  (params (OtherActor :type Actor%20Object%20Reference)))

(event EventTick
  (params (DeltaSeconds :type Float%20%28single-precision%29)))

(fn ConstructionScript
  (bind _curve_along_spline (Variables|Configuration|GetCurve%20Along%20Spline))
  (bind _returnvalue (not _curve_along_spline))
  (Variables|Random|SetRandom%20Stream (Math|Random|MakeRandomStream (Variables|Random|GetRandom%20Seed)))
  (if (Variables|Configuration|GetUniform%20Distribution)
    (for _index (range 1 (Variables|Configuration|GetNumber%20Of%20Meshes))
      (LocalVariables|SetCurrent%20Index _index)
      (Utilities|FlowControl|Sequence
        (:then_0
          ;[1 1 1] Random mesh select
          (switch int (LocalVariables|GetCurrent%20Index)
            (:Default
              (if (or (== (LocalVariables|GetCurrent%20Index) (Variables|Configuration|GetNumber%20Of%20Meshes)) (> (+ (LocalVariables|GetCurrent%20Spline%20Length%20Position) (Variables|Configuration|GetMinimum%20Mesh%20Width)) (Spline|GetSplineLength (Variables|Components|GetSpline))))
                (bind (_mesh_instance _local_transform _mesh_width _mesh_static) (Generators|GetMesh "NewEnumerator2" _returnvalue))
                (LocalVariables|SetSelected%20Mesh%20Instance _mesh_instance)
                (LocalVariables|SetSelected%20Mesh%20Local%20Transform _local_transform)
                (LocalVariables|SetSelected%20Mesh%20Width _mesh_width)
                (LocalVariables|SetSelected%20Mesh _mesh_static)
                (else
                  (bind (_mesh_instance_2 _local_transform_2 _mesh_width_2 _mesh_static_2) (Generators|GetMesh "NewEnumerator1" _returnvalue))
                  (LocalVariables|SetSelected%20Mesh%20Instance _mesh_instance_2)
                  (LocalVariables|SetSelected%20Mesh%20Local%20Transform _local_transform_2)
                  (LocalVariables|SetSelected%20Mesh%20Width _mesh_width_2)
                  (LocalVariables|SetSelected%20Mesh _mesh_static_2))))
            (:1
              (bind (_mesh_instance_3 _local_transform_3 _mesh_width_3 _mesh_static_3) (Generators|GetMesh "NewEnumerator0" _returnvalue))
              (LocalVariables|SetSelected%20Mesh%20Instance _mesh_instance_3)
              (LocalVariables|SetSelected%20Mesh%20Local%20Transform _local_transform_3)
              (LocalVariables|SetSelected%20Mesh%20Width _mesh_width_3)
              (LocalVariables|SetSelected%20Mesh _mesh_static_3))))
        (:then_1
          ;[1 1 1] Get main transform
          (bind _result_transform (Generators|GetTransform (Variables|Configuration|GetUniform%20Distribution) (LocalVariables|GetCurrent%20Index) (Variables|Configuration|GetNumber%20Of%20Meshes) (LocalVariables|GetCurrent%20Spline%20Length%20Position) (LocalVariables|GetSelected%20Mesh%20Local%20Transform)))
          (LocalVariables|SetDesired%20Transform _result_transform)
          (LocalVariables|SetCurrent%20Spline%20Length%20Position (+ (LocalVariables|GetCurrent%20Spline%20Length%20Position) (Math|Float|Max(Float) (LocalVariables|GetSelected%20Mesh%20Width) (Variables|Configuration|GetMinimum%20Mesh%20Width))))
          ;[1 1 1] Face next mesh rotation
          (if (Variables|Configuration|GetFace%20Next%20Mesh%20Rotation)
            (bind _result_transform_2 (Generators|GetTransform (Variables|Configuration|GetUniform%20Distribution) (+ (LocalVariables|GetCurrent%20Index) 1) (Variables|Configuration|GetNumber%20Of%20Meshes) (LocalVariables|GetCurrent%20Spline%20Length%20Position) (LocalVariables|GetSelected%20Mesh%20Local%20Transform)))
            (LocalVariables|SetDesired%20Transform (Math|Transform|MakeTransform (.location (LocalVariables|GetDesired%20Transform)) (Math|Rotator|MakeRotator (Math|Float|SelectFloat (.Roll (Math|Rotator|BreakRotator (.rotation (LocalVariables|GetDesired%20Transform)))) (.roll (Math|Rotator|CombineRotators (.rotation (LocalVariables|GetDesired%20Transform)) (Math|Rotator|MakeRotfromX (- (.location _result_transform_2) (.location (LocalVariables|GetDesired%20Transform)))))) (Variables|Configuration|GetAllow%20Face%20Yaw%20Only)) (Math|Float|SelectFloat (.Pitch (Math|Rotator|BreakRotator (.rotation (LocalVariables|GetDesired%20Transform)))) (.pitch (Math|Rotator|CombineRotators (.rotation (LocalVariables|GetDesired%20Transform)) (Math|Rotator|MakeRotfromX (- (.location _result_transform_2) (.location (LocalVariables|GetDesired%20Transform)))))) (Variables|Configuration|GetAllow%20Face%20Yaw%20Only)) (.yaw (Math|Rotator|CombineRotators (.rotation (LocalVariables|GetDesired%20Transform)) (Math|Rotator|MakeRotfromX (- (.location _result_transform_2) (.location (LocalVariables|GetDesired%20Transform))))))) (.scale (LocalVariables|GetDesired%20Transform))))))
        (:then_2
          (if (Variables|Configuration|GetCurve%20Along%20Spline)
            ;[1 1 1] Spline mesh generation
            (bind _returnvalue_2 (AddComponent|AddSplineMeshComponent false))
            (Components|StaticMesh|SetStaticMesh _returnvalue_2 (LocalVariables|GetSelected%20Mesh))
            (bind _result_transform_3 (Generators|GetTransform (Variables|Configuration|GetUniform%20Distribution) (+ (LocalVariables|GetCurrent%20Index) 1) (Variables|Configuration|GetNumber%20Of%20Meshes) (LocalVariables|GetCurrent%20Spline%20Length%20Position) (LocalVariables|GetSelected%20Mesh%20Local%20Transform)))
            (SplineMesh|SetStartandEnd _returnvalue_2 (.location (LocalVariables|GetDesired%20Transform)) (* (* (Math|Vector|GetForwardVector (.rotation (LocalVariables|GetDesired%20Transform))) (Math|Float|SelectFloat (/ (Spline|GetSplineLength (Variables|Components|GetSpline)) (Math|Conversions|ToFloat(Integer) (Math|Integer|Max(Integer) (Variables|Configuration|GetNumber%20Of%20Meshes) 1))) (LocalVariables|GetSelected%20Mesh%20Width) (Variables|Configuration|GetUniform%20Distribution))) (.scale (LocalVariables|GetDesired%20Transform))) (.location _result_transform_3) (* (* (Math|Vector|GetForwardVector (.rotation _result_transform_3)) (Math|Float|SelectFloat (/ (Spline|GetSplineLength (Variables|Components|GetSpline)) (Math|Conversions|ToFloat(Integer) (Math|Integer|Max(Integer) (Variables|Configuration|GetNumber%20Of%20Meshes) 1))) (LocalVariables|GetSelected%20Mesh%20Width) (Variables|Configuration|GetUniform%20Distribution))) (.scale _result_transform_3)) true :!class /Script/Engine.SplineMeshComponent)
            ;[1 1 1] Spline curve scale
            (SplineMesh|SetStartScale _returnvalue_2 (Math|Vector2D|MakeVector2D (.Y (Math|Vector|BreakVector (.scale (LocalVariables|GetDesired%20Transform)))) (.Z (Math|Vector|BreakVector (.scale (LocalVariables|GetDesired%20Transform))))) true :!class /Script/Engine.SplineMeshComponent)
            (SplineMesh|SetEndScale _returnvalue_2 (Math|Vector2D|MakeVector2D (.Y (Math|Vector|BreakVector (.scale _result_transform_3))) (.Z (Math|Vector|BreakVector (.scale _result_transform_3)))) true :!class /Script/Engine.SplineMeshComponent)
            (else
              (Components|InstancedStaticMesh|AddInstance (LocalVariables|GetSelected%20Mesh%20Instance) (LocalVariables|GetDesired%20Transform) false))))))
    (else
      (LocalVariables|SetCurrent%20Spline%20Length%20Position 0.0)
      (LocalVariables|SetCurrent%20Index 0)
      (while (and (<= (LocalVariables|GetCurrent%20Spline%20Length%20Position) (Spline|GetSplineLength (Variables|Components|GetSpline))) (< (LocalVariables|GetCurrent%20Index) (Variables|Configuration|GetNumber%20Of%20Meshes)))
        (Math|Integer|IncrementInt (LocalVariables|GetCurrent%20Index)
          (:%20%20
            (Utilities|FlowControl|Sequence
              (:then_0
                (switch int (LocalVariables|GetCurrent%20Index)
                  (:Default
                    (if (or (== (LocalVariables|GetCurrent%20Index) (Variables|Configuration|GetNumber%20Of%20Meshes)) (> (+ (LocalVariables|GetCurrent%20Spline%20Length%20Position) (Variables|Configuration|GetMinimum%20Mesh%20Width)) (Spline|GetSplineLength (Variables|Components|GetSpline))))
                      (bind (_mesh_instance_4 _local_transform_4 _mesh_width_4 _mesh_static_4) (Generators|GetMesh "NewEnumerator2" _returnvalue))
                      (LocalVariables|SetSelected%20Mesh%20Instance _mesh_instance_4)
                      (LocalVariables|SetSelected%20Mesh%20Local%20Transform _local_transform_4)
                      (LocalVariables|SetSelected%20Mesh%20Width _mesh_width_4)
                      (LocalVariables|SetSelected%20Mesh _mesh_static_4)
                      (else
                        (bind (_mesh_instance_5 _local_transform_5 _mesh_width_5 _mesh_static_5) (Generators|GetMesh "NewEnumerator1" _returnvalue))
                        (LocalVariables|SetSelected%20Mesh%20Instance _mesh_instance_5)
                        (LocalVariables|SetSelected%20Mesh%20Local%20Transform _local_transform_5)
                        (LocalVariables|SetSelected%20Mesh%20Width _mesh_width_5)
                        (LocalVariables|SetSelected%20Mesh _mesh_static_5))))
                  (:1
                    (bind (_mesh_instance_6 _local_transform_6 _mesh_width_6 _mesh_static_6) (Generators|GetMesh "NewEnumerator0" _returnvalue))
                    (LocalVariables|SetSelected%20Mesh%20Instance _mesh_instance_6)
                    (LocalVariables|SetSelected%20Mesh%20Local%20Transform _local_transform_6)
                    (LocalVariables|SetSelected%20Mesh%20Width _mesh_width_6)
                    (LocalVariables|SetSelected%20Mesh _mesh_static_6))))
              (:then_1
                (bind _result_transform_4 (Generators|GetTransform (Variables|Configuration|GetUniform%20Distribution) (LocalVariables|GetCurrent%20Index) (Variables|Configuration|GetNumber%20Of%20Meshes) (LocalVariables|GetCurrent%20Spline%20Length%20Position) (LocalVariables|GetSelected%20Mesh%20Local%20Transform)))
                (LocalVariables|SetDesired%20Transform _result_transform_4)
                (LocalVariables|SetCurrent%20Spline%20Length%20Position (+ (LocalVariables|GetCurrent%20Spline%20Length%20Position) (Math|Float|Max(Float) (LocalVariables|GetSelected%20Mesh%20Width) (Variables|Configuration|GetMinimum%20Mesh%20Width))))
                (if (Variables|Configuration|GetFace%20Next%20Mesh%20Rotation)
                  (bind _result_transform_5 (Generators|GetTransform (Variables|Configuration|GetUniform%20Distribution) (+ (LocalVariables|GetCurrent%20Index) 1) (Variables|Configuration|GetNumber%20Of%20Meshes) (LocalVariables|GetCurrent%20Spline%20Length%20Position) (LocalVariables|GetSelected%20Mesh%20Local%20Transform)))
                  (LocalVariables|SetDesired%20Transform (Math|Transform|MakeTransform (.location (LocalVariables|GetDesired%20Transform)) (Math|Rotator|MakeRotator (Math|Float|SelectFloat (.Roll (Math|Rotator|BreakRotator (.rotation (LocalVariables|GetDesired%20Transform)))) (.roll (Math|Rotator|CombineRotators (.rotation (LocalVariables|GetDesired%20Transform)) (Math|Rotator|MakeRotfromX (- (.location _result_transform_5) (.location (LocalVariables|GetDesired%20Transform)))))) (Variables|Configuration|GetAllow%20Face%20Yaw%20Only)) (Math|Float|SelectFloat (.Pitch (Math|Rotator|BreakRotator (.rotation (LocalVariables|GetDesired%20Transform)))) (.pitch (Math|Rotator|CombineRotators (.rotation (LocalVariables|GetDesired%20Transform)) (Math|Rotator|MakeRotfromX (- (.location _result_transform_5) (.location (LocalVariables|GetDesired%20Transform)))))) (Variables|Configuration|GetAllow%20Face%20Yaw%20Only)) (.yaw (Math|Rotator|CombineRotators (.rotation (LocalVariables|GetDesired%20Transform)) (Math|Rotator|MakeRotfromX (- (.location _result_transform_5) (.location (LocalVariables|GetDesired%20Transform))))))) (.scale (LocalVariables|GetDesired%20Transform))))))
              (:then_2
                (if (Variables|Configuration|GetCurve%20Along%20Spline)
                  (bind _returnvalue_3 (AddComponent|AddSplineMeshComponent false))
                  (Components|StaticMesh|SetStaticMesh _returnvalue_3 (LocalVariables|GetSelected%20Mesh))
                  (bind _result_transform_6 (Generators|GetTransform (Variables|Configuration|GetUniform%20Distribution) (+ (LocalVariables|GetCurrent%20Index) 1) (Variables|Configuration|GetNumber%20Of%20Meshes) (LocalVariables|GetCurrent%20Spline%20Length%20Position) (LocalVariables|GetSelected%20Mesh%20Local%20Transform)))
                  (SplineMesh|SetStartandEnd _returnvalue_3 (.location (LocalVariables|GetDesired%20Transform)) (* (* (Math|Vector|GetForwardVector (.rotation (LocalVariables|GetDesired%20Transform))) (Math|Float|SelectFloat (/ (Spline|GetSplineLength (Variables|Components|GetSpline)) (Math|Conversions|ToFloat(Integer) (Math|Integer|Max(Integer) (Variables|Configuration|GetNumber%20Of%20Meshes) 1))) (LocalVariables|GetSelected%20Mesh%20Width) (Variables|Configuration|GetUniform%20Distribution))) (.scale (LocalVariables|GetDesired%20Transform))) (.location _result_transform_6) (* (* (Math|Vector|GetForwardVector (.rotation _result_transform_6)) (Math|Float|SelectFloat (/ (Spline|GetSplineLength (Variables|Components|GetSpline)) (Math|Conversions|ToFloat(Integer) (Math|Integer|Max(Integer) (Variables|Configuration|GetNumber%20Of%20Meshes) 1))) (LocalVariables|GetSelected%20Mesh%20Width) (Variables|Configuration|GetUniform%20Distribution))) (.scale _result_transform_6)) true :!class /Script/Engine.SplineMeshComponent)
                  (SplineMesh|SetStartScale _returnvalue_3 (Math|Vector2D|MakeVector2D (.Y (Math|Vector|BreakVector (.scale (LocalVariables|GetDesired%20Transform)))) (.Z (Math|Vector|BreakVector (.scale (LocalVariables|GetDesired%20Transform))))) true :!class /Script/Engine.SplineMeshComponent)
                  (SplineMesh|SetEndScale _returnvalue_3 (Math|Vector2D|MakeVector2D (.Y (Math|Vector|BreakVector (.scale _result_transform_6))) (.Z (Math|Vector|BreakVector (.scale _result_transform_6)))) true :!class /Script/Engine.SplineMeshComponent)
                  (else
                    (Components|InstancedStaticMesh|AddInstance (LocalVariables|GetSelected%20Mesh%20Instance) (LocalVariables|GetDesired%20Transform) false)))))))))))

(fn GetMesh
  (params (Section :type SplineSection%20Enum :default "NewEnumerator0") (Instance%20Mesh :type Boolean))
  (bind _end_meshes (Variables|Assets|GetEnd%20Meshes))
  (bind _start_meshes (Variables|Assets|GetStart%20Meshes))
  (LocalVariables|SetCreate%20Instance Instance%20Mesh)
  (switch Utilities|FlowControl|Switch|SwitchonSplineSection Section
    (:NewEnumerator0
      (if (> (Utilities|Array|Length _start_meshes) 0)
        (LocalVariables|SetSelected%20Meshes _start_meshes)
        (else
          (LocalVariables|SetSelected%20Meshes (Variables|Assets|GetFill%20Meshes) :!label _label))))
    (:NewEnumerator1
      (goto _label))
    (:NewEnumerator2
      (if (> (Utilities|Array|Length _end_meshes) 0)
        (LocalVariables|SetSelected%20Meshes _end_meshes)
        (else
          (goto _label)))))
  (if (> (Utilities|Array|Length (LocalVariables|GetSelected%20Meshes)) 0)
    (LocalVariables|SetSelected%20Spline%20Mesh (Utilities|Array|Get(acopy) (LocalVariables|GetSelected%20Meshes) (Math|Random|RandomIntegerinRangefromStream (Variables|Random|GetRandom%20Stream) 0 (- (Utilities|Array|Length (LocalVariables|GetSelected%20Meshes)) 1))))
    (if (LocalVariables|GetCreate%20Instance)
      (bind _array_element (Utilities|Array|ForEachLoopwithBreak (Actor|GetComponentsByClass "/Script/Engine.InstancedStaticMeshComponent"))
        (:LoopBody
          (if (== (Variables|/Script/Engine.StaticMeshComponent|GetStaticMesh _array_element) (.mesh (LocalVariables|GetSelected%20Spline%20Mesh)))
            (return _array_element (.transform (LocalVariables|GetSelected%20Spline%20Mesh)) (.width (LocalVariables|GetSelected%20Spline%20Mesh)) (.mesh (LocalVariables|GetSelected%20Spline%20Mesh)))))
        (:Completed
          (bind _returnvalue (AddComponent|AddInstancedStaticMeshComponent false))
          (Components|StaticMesh|SetStaticMesh _returnvalue (.mesh (LocalVariables|GetSelected%20Spline%20Mesh)))
          (return _returnvalue (.transform (LocalVariables|GetSelected%20Spline%20Mesh)) (.width (LocalVariables|GetSelected%20Spline%20Mesh)) (.mesh (LocalVariables|GetSelected%20Spline%20Mesh)))))
      (else
        (return 0 (.transform (LocalVariables|GetSelected%20Spline%20Mesh)) (.width (LocalVariables|GetSelected%20Spline%20Mesh)) (.mesh (LocalVariables|GetSelected%20Spline%20Mesh)))))
    (else
      (return 0 "" (Variables|Configuration|GetMinimum%20Mesh%20Width) (Variables|Assets|GetDefault%20Static%20Mesh)))))

(fn GetTransform
  (params (Is%20Uniform :type Boolean) (Current%20Index :type Integer) (Max%20Index :type Integer) (Spline%20Length%20Position :type Float%20%28double-precision%29) (Mesh%20Local%20Transform :type Transform))
  (bind _random_stream (Variables|Random|GetRandom%20Stream))
  (bind _random_offset_variations (Variables|Random|GetRandom%20Offset%20Variations))
  (bind _random_offset (Variables|Random|GetRandom%20Offset))
  (bind _random_stream_2 (Variables|Random|GetRandom%20Stream))
  (bind _random_rotation_variations (Variables|Random|GetRandom%20Rotation%20Variations))
  (bind _returnvalue (Math|Random|RandomUnitVectorfromStream _random_stream))
  (bind _returnvalue_2 (Math|Random|RandomUnitVectorfromStream _random_stream_2))
  (bind _returnvalue_3 (* _returnvalue_2 _random_offset_variations))
  (bind _returnvalue_4 (* _returnvalue _random_rotation_variations))
  (bind _returnvalue_5 (Math|Vector|SelectVector _returnvalue_3 "0, 0, 0" _random_offset))
  (LocalVariables|SetUniform%20Dist Is%20Uniform)
  (LocalVariables|SetMesh%20Index Current%20Index)
  (LocalVariables|SetMesh%20Count Max%20Index)
  (LocalVariables|SetSpline%20Position Spline%20Length%20Position)
  (LocalVariables|SetMesh%20Transform Mesh%20Local%20Transform)
  (Utilities|FlowControl|Sequence
    (:then_0
      ;[1 1 1] Spline position calculation
      (if (LocalVariables|GetUniform%20Dist)
        (LocalVariables|SetSpline%20Point%20Transform (Spline|GetTransformatDistanceAlongSpline (Variables|Components|GetSpline) (* (- (LocalVariables|GetMesh%20Index) 1) (/ (Spline|GetSplineLength (Variables|Components|GetSpline)) (Math|Conversions|ToFloat(Integer) (Math|Integer|Max(Integer) (- (LocalVariables|GetMesh%20Count) (Math|Integer|SelectInt 0 1 (Variables|Configuration|GetCurve%20Along%20Spline))) 1)))) "Local" true))
        (else
          (LocalVariables|SetSpline%20Point%20Transform (Spline|GetTransformatDistanceAlongSpline (Variables|Components|GetSpline) (LocalVariables|GetSpline%20Position) "Local" true)))))
    (:then_1
      ;[1 1 1] Apply transform modifications
      (LocalVariables|SetDesired%20Transform (Math|Transform|MakeTransform (.Location (Math|Transform|BreakTransform (LocalVariables|GetSpline%20Point%20Transform))) (Math|Rotator|SelectRotator (.Rotation (Math|Transform|BreakTransform (LocalVariables|GetSpline%20Point%20Transform))) "0, 0, 0" (Variables|Configuration|GetRotate%20Along%20Spline)) (Math|Vector|SelectVector (.Scale (Math|Transform|BreakTransform (LocalVariables|GetSpline%20Point%20Transform))) "1.000000,1.000000,1.000000" (Variables|Configuration|GetScale%20Along%20Spline))))
      ;[1 1 1] Yaw Only Rotation
      (if (Variables|Configuration|GetAllow%20Spline%20Yaw%20Only)
        (LocalVariables|SetDesired%20Transform (Math|Transform|MakeTransform (.location (LocalVariables|GetDesired%20Transform)) (Math|Rotator|MakeRotator 0.0 0.0 (.yaw (.rotation (LocalVariables|GetDesired%20Transform)))) (.scale (LocalVariables|GetDesired%20Transform)))))
      ;[1 1 1] Local Mesh Transform
      (if (Variables|Configuration|GetLocal%20Transform%20Enabled)
        (LocalVariables|SetDesired%20Transform (Math|Transform|ComposeTransforms (Math|Transform|MakeTransform (Math|Vector|SelectVector (.location (LocalVariables|GetMesh%20Transform)) (Math|Vector|RotateVector (.location (LocalVariables|GetMesh%20Transform)) (.rotation (LocalVariables|GetSpline%20Point%20Transform))) (Variables|Configuration|GetRotate%20Along%20Spline)) (.rotation (LocalVariables|GetMesh%20Transform)) (.scale (LocalVariables|GetMesh%20Transform))) (LocalVariables|GetDesired%20Transform)))))
    (:then_2
      ;[1 1 1] Random
      (LocalVariables|SetDesired%20Transform (Math|Transform|ComposeTransforms (Math|Transform|MakeTransform (Math|Vector|SelectVector _returnvalue_5 (Math|Vector|RotateVector _returnvalue_5 (.rotation (LocalVariables|GetSpline%20Point%20Transform))) (Variables|Configuration|GetRotate%20Along%20Spline)) (Math|Rotator|SelectRotator (Math|Rotator|MakeRotator (.x _returnvalue_4) (.y _returnvalue_4) (.z _returnvalue_4)) "0, 0, 0" (Variables|Random|GetRandom%20Rotation)) (* (Math|Vector|MakeVector 1.0 1.0 1.0) (Math|Float|SelectFloat (Math|Random|RandomFloatinRangefromStream (Variables|Random|GetRandom%20Stream) (Variables|Random|GetRandom%20Scale%20Min) (Variables|Random|GetRandom%20Scale%20Max)) 1.0 (Variables|Random|GetRandom%20Scale)))) (LocalVariables|GetDesired%20Transform))))
    (:then_3
      ;[1 1 1] Snap to Terrain
      (if (Variables|Configuration|GetSnap%20To%20Terrain)
        (bind (_outhit _returnvalue_6) (Collision|LineTraceByChannel (+ (Transformation|GetActorLocation) (.Location (Math|Transform|BreakTransform (LocalVariables|GetDesired%20Transform)))) (- (+ (Transformation|GetActorLocation) (.Location (Math|Transform|BreakTransform (LocalVariables|GetDesired%20Transform)))) (Math|Vector|MakeVector 0.0 0.0 (Variables|Configuration|GetTerrain%20Trace%20Depth))) "TraceTypeQuery1" true 0 "ForDuration"))
        (if _returnvalue_6
          (LocalVariables|SetDesired%20Transform (Math|Transform|MakeTransform (- (.ImpactPoint (Collision|BreakHitResult _outhit)) (Transformation|GetActorLocation)) (.rotation (LocalVariables|GetDesired%20Transform)) (.scale (LocalVariables|GetDesired%20Transform)))))))
    (:then_4
      (return (LocalVariables|GetDesired%20Transform)))))